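; BP_PinchoMovil is a moving spike hazard that kills the player on contact.
; The construction script gives its InterpToMovement component two relative control points, the origin and the Pos variable, to define its path.
; When Box1 overlaps BP_ThirdPersonCharacter, it shows the WBP_MenuMuerte death menu, pauses the game, destroys the character and switches to UI-only input with a visible cursor.
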(event `self.Box1.OnComponentBeginOverlap`
  (params (OverlappedComponent :type "PrimitiveComponent Object Reference") (OtherActor :type "Actor Object Reference") (OtherComp :type "PrimitiveComponent Object Reference") (OtherBodyIndex :type Integer) (bFromSweep :type Boolean) (SweepResult :type "HitResult Structure (by ref)"))
  (bind _returnvalue (`GameplayStatics.GetPlayerController` 0))
  ; Logica del Pincho de muerte
  (bind _asbp_third_person_character (cast `/Game/ThirdPerson/Blueprints/BP_ThirdPersonCharacter` OtherActor))
  (bind _returnvalue_2 (`|CreateWidget` "/Game/UI/WBP_MenuMuerte.WBP_MenuMuerte_C"))
  (`UserWidget.AddToViewport` _returnvalue_2 0)
  (`GameplayStatics.SetGamePaused` true)
  (`self.K2_DestroyActor` _asbp_third_person_character)
  (set `PlayerController.bShowMouseCursor` true _returnvalue)
  (`WidgetBlueprintLibrary.SetInputMode_UIOnlyEx` _returnvalue _returnvalue_2))

(fn `UserConstructionScript`
  (`InterpToMovementComponent.AddControlPointPosition` (`self.InterpToMovement`) (0.0 0.0 0.0) true)
  (`InterpToMovementComponent.AddControlPointPosition` (`self.InterpToMovement`) (`self.Pos`) true))