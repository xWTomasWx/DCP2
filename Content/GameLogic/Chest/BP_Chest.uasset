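; BP_Chest is an interactable treasure chest that opens once and randomly gives the player either a key or coins.
; Interact plays a timeline swinging two doors in mirrored yaw, with a delay chained from its update that marks it opened and grants the reward.
; An overlap box enables input and shows an Interfaz widget while unopened, undoing both when the character leaves.
; CanInteract reports whether the chest is still closed.
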(event `/Game/GameLogic/Chest/BPI_Interactable.Interact`
  (params (Caller :type "Actor Object Reference"))
  (if (not (`self.bOpened`))
    (bind (_direction _apertura) (`Timeline|Timeline` :!via `PlayFromStart`)
      (:`Update`
        (bind _returnvalue (`KismetMathLibrary.MakeRotator` 0.0 0.0 (`KismetMathLibrary.Lerp` 0.0 -110.0 _apertura)))
        (`SceneComponent.K2_SetRelativeRotation` (`self.DoorRight`) _returnvalue false false)
        (`SceneComponent.K2_SetRelativeRotation` (`self.DoorLeft`) (`KismetMathLibrary.NegateRotator` _returnvalue) false false)
        (`KismetSystemLibrary.Delay` 1.5)
        (set `self.bOpened` true)
        (if (== (`KismetMathLibrary.RandomIntegerInRange` 0 1) 0)
          (bind _asbp_third_person_character (cast `/Game/ThirdPerson/Blueprints/BP_ThirdPersonCharacter` (`GameplayStatics.GetPlayerCharacter` 0)))
          (`KismetArrayLibrary.Array_Add` (`/Game/ThirdPerson/Blueprints/BP_ThirdPersonCharacter.KeysInventory` _asbp_third_person_character) "NewEnumerator0")
          (`KismetSystemLibrary.PrintString` "Consiguio la llave")
          (else
            (bind _asbp_third_person_character_2 (cast `/Game/ThirdPerson/Blueprints/BP_ThirdPersonCharacter` (`GameplayStatics.GetPlayerCharacter` 0)))
            (bind _output_get (set `/Game/ThirdPerson/Blueprints/BP_ThirdPersonCharacter.Coins` (+ (`self.CoinsToGive`) (`/Game/ThirdPerson/Blueprints/BP_ThirdPersonCharacter.Coins` _asbp_third_person_character_2)) _asbp_third_person_character_2))
            (`KismetSystemLibrary.PrintString` (`KismetStringLibrary.Conv_IntToString` _output_get))))))))

(event `self.BoxText.OnComponentBeginOverlap`
  (params (OverlappedComponent :type "PrimitiveComponent Object Reference") (OtherActor :type "Actor Object Reference") (OtherComp :type "PrimitiveComponent Object Reference") (OtherBodyIndex :type Integer) (bFromSweep :type Boolean) (SweepResult :type "HitResult Structure (by ref)"))
  (if (not (`self.bOpened`))
    (cast `/Game/ThirdPerson/Blueprints/BP_ThirdPersonCharacter` OtherActor)
    (`self.EnableInput` (`GameplayStatics.GetPlayerController` 0))
    (bind _returnvalue (`|CreateWidget` "/Game/GameLogic/Tools/NormalDoor/Interfaz.Interfaz_C"))
    (`UserWidget.AddToViewport` _returnvalue 0)))

(event `self.BoxText.OnComponentEndOverlap`
  (params (OverlappedComponent :type "PrimitiveComponent Object Reference") (OtherActor :type "Actor Object Reference") (OtherComp :type "PrimitiveComponent Object Reference") (OtherBodyIndex :type Integer))
  (cast `/Game/ThirdPerson/Blueprints/BP_ThirdPersonCharacter` OtherActor)
  (`self.DisableInput` null)
  (bind _foundwidgets (`WidgetBlueprintLibrary.GetAllWidgetsOfClass` "/Game/GameLogic/Tools/NormalDoor/Interfaz.Interfaz_C"))
  (`Widget.RemoveFromParent` _foundwidgets))

(fn `CanInteract`
  (params (Caller :type "Actor Object Reference"))
  (returns (ReturnValue :type Boolean))
  (return (not (`self.bOpened`))))

(fn `UserConstructionScript`)